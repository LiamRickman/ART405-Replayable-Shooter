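; Base first-person gun actor, used as a child actor of FPS_Character, handling firing, ammo and reloading.
; Construction attaches the gun mesh to the arms' grip socket, and start/stop events only toggle a firing flag.
; Hitscan fire, blocked while reloading, spends ammo and traces from the camera, spawning explosion effects and pushing physics objects.
; A timed reload refills from reserve ammo; a projectile-fire function exists but is not called here.
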(event Custom|StartShooting
  (Variables|Default|SetIsFiring true))

(event Custom|StopShooting
  (Variables|Default|SetIsFiring false))

(event Custom|FireHitscan
  (if (not (Variables|Default|GetReloading))
    (CallFunction|FireHitscanBullet)))

(event Custom|Reload
  (Utilities|DoReload))

(fn ConstructionScript
  (Transformation|AttachComponentToComponent (Variables|Default|GetGuns) (Variables|Default|GetArms) "GripPoint" "SnapToTarget" "SnapToTarget" "SnapToTarget" true))

(fn FireProjectileBullet
  (bind _asfps_character (Utilities|Casting|CastToFPS_Character (Actor|GetParentActor)))
  (if (> (Variables|Default|GetCurrentAmmo) 0)
    (Audio|PlaySoundatLocation "/Game/SFX/Weapons/Gunshot.Gunshot" (Transformation|GetActorLocation) "0, 0, 0" 1.0 1.0 0.0 0 0 0 0)
    (Game|SpawnActorfromClass "/Game/FirstPerson/Blueprints/BP_FirstPersonProjectile.BP_FirstPersonProjectile_C" (Math|Transform|MakeTransform (Transformation|GetWorldLocation (Variables|Default|GetBarrelRef)) (Transformation|GetWorldRotation (Variables|/Game/Blueprints/PlayerCharacter/FPS_Character.FPS_Character_C|GetCamera _asfps_character)) "1.000000,1.000000,1.000000") "Undefined" 0 0)
    (Animation|Montage|MontagePlay (Components|SkeletalMesh|GetAnimInstance (Variables|Default|GetArms)) "/Game/FirstPersonArms/Animations/FirstPersonFire_Montage.FirstPersonFire_Montage" 1.0 "MontageLength" 0.0 true)))

(fn FireHitscanBullet
  (bind _asfps_character (Utilities|Casting|CastToFPS_Character (Actor|GetParentActor)))
  (if (> (Variables|Default|GetCurrentAmmo) 0)
    (Audio|PlaySoundatLocation (Variables|Default|GetGunShotSFX) (Transformation|GetActorLocation) "0, 0, 0" 1.0 1.0 0.0 0 0 0 0)
    (Animation|Montage|MontagePlay (Components|SkeletalMesh|GetAnimInstance (Variables|Default|GetArms)) "/Game/FirstPersonArms/Animations/FirstPersonFire_Montage.FirstPersonFire_Montage" 1.0 "MontageLength" 0.0 true)
    (Math|Integer|DecrementInt (Variables|Default|GetCurrentAmmo)
      (:%20%20
        (bind (_outhit _returnvalue) (Collision|LineTraceForObjects (Transformation|GetWorldLocation (Variables|/Game/Blueprints/PlayerCharacter/FPS_Character.FPS_Character_C|GetCamera _asfps_character)) (+ (Transformation|GetWorldLocation (Variables|/Game/Blueprints/PlayerCharacter/FPS_Character.FPS_Character_C|GetCamera _asfps_character)) (* (Math|Vector|GetForwardVector (Transformation|GetWorldRotation (Variables|/Game/Blueprints/PlayerCharacter/FPS_Character.FPS_Character_C|GetCamera _asfps_character))) (Variables|Default|GetShotRange))) (Utilities|Array|MakeArray "ObjectTypeQuery1" "ObjectTypeQuery4") false 0 "None" true "(R=1.000000,G=0.000000,B=0.000000,A=1.000000)" "(R=0.000000,G=1.000000,B=0.000000,A=1.000000)" 0.5))
        (if _returnvalue
          (Effects|SpawnEmitteratLocation "/Game/StarterContent/Particles/P_Explosion.P_Explosion" (.Location (Collision|BreakHitResult _outhit)))
          (if (Physics|IsSimulatingPhysics (Variables|/Script/Engine.Actor|GetRootComponent (.HitActor (Collision|BreakHitResult _outhit))) "None")
            (Physics|AddImpulseatLocation (.HitComponent (Collision|BreakHitResult _outhit)) (* (Math|Vector|GetForwardVector (Transformation|GetWorldRotation (Variables|/Game/Blueprints/PlayerCharacter/FPS_Character.FPS_Character_C|GetCamera _asfps_character))) (Variables|Default|GetImpulseStrength)) (.Location (Collision|BreakHitResult _outhit)) "None")))))))