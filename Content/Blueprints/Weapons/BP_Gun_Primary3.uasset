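; BP_Gun_Primary3 is a child gun Blueprint for a primary weapon that fires automatic hitscan shots.
; StartShooting calls the parent, then with ammo fires immediately and starts a looping FireRate timer that repeats FireHitscan, or reloads when empty.
; StopShooting calls the parent and clears the timer, while the Reload input also triggers a reload.
; Ammo is checked only when shooting starts, not on each timer tick in this graph.
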(event Custom|Fire
  (CallFunction|FireHitscan))

(event EventStartShooting
  (|CallParentFunction)
  (if (> (Variables|Default|GetCurrentAmmo) 0)
    (CallFunction|FireHitscan)
    (bind _returnvalue (Utilities|Time|SetTimerbyEvent (delegate Custom|Fire) (Variables|Default|GetFireRate) true))
    (Variables|Default|SetGunTimer _returnvalue)
    (else
      (CallFunction|Reload))))

(event EventStopShooting
  (|CallParentFunction)
  (Utilities|Time|ClearandInvalidateTimerbyHandle (Variables|Default|GetGunTimer)))

(event Input|ActionEvents|InputActionReload
  (params (Key :type Key%20Structure :default "None"))
  (:Pressed
    (CallFunction|Reload)))

(fn ConstructionScript
  (|CallParentFunction))