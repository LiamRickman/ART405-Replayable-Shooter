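; Procedural room actor that builds a tiled floor and perimeter walls from instances, with BP_Door actors spawned at random eligible slots.
; BasicRoom runs on construction and BeginPlay, using a seeded stream and modulo spacing to pick doors, and leaving an entry gap in non-origin rooms.
; UnderConstructionRoom, uncalled here, adds entry shift, hall and door seeding support.
; RemoveWall deletes WallH instances, swap-removing their collision entries to keep indices aligned.
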(event Custom|RemoveWall
  (params (Index :type Integer))
  (bind _wallcollisions (Variables|Default|GetWallCollisions))
  (bind _returnvalue (Utilities|Array|LastIndex _wallcollisions))
  (bind _output (Utilities|Array|Get(acopy) _wallcollisions _returnvalue))
  (Class|InstancedStaticMeshComponent|RemoveInstance (Variables|Default|GetWall_H) Index)
  (Utilities|Array|SetArrayElem _wallcollisions Index _output)
  (Default|Update _output Index)
  (Utilities|Array|RemoveIndex (Variables|Default|GetWallCollisions) Index))

(event EventBeginPlay
  (CallFunction|BasicRoom))

(fn ConstructionScript
  (Utilities|Array|Clear (Variables|RoomSize|GetDoors))
  (CallFunction|BasicRoom))

(fn BasicRoom
  ;[1 1 1] Floor generation
  (for _index (range 0 (- (Variables|RoomSize|GetRoomTilesY) 1))
    (for _index_2 (range 0 (- (Variables|RoomSize|GetRoomTilesX) 1))
      (Components|InstancedStaticMesh|AddInstance (Variables|Default|GetFloor) (Math|Transform|MakeTransform (Math|Vector|MakeVector (* (Math|Conversions|ToFloat(Integer) _index_2) (Variables|RoomSize|GetTileSizeX)) (* (Math|Conversions|ToFloat(Integer) _index) (Variables|RoomSize|GetTileSizeY)) 0.0) "0, 0, 0" "1.000000,1.000000,1.000000") false)))
  (for _index_3 (range 0 (- (Variables|RoomSize|GetRoomTilesY) 1))
    ;[1 1 1] IsFirstRoom?
    (if (or (Variables|Default|GetOrigin) (!= _index_3 0))
      ;[1 1 1] Bottom Wall
      (CallFunction|WallorDoor (== (Math|Integer|%(Integer) _index_3 (Variables|Default|GetDoor%20Every)) (Variables|Default|GetDoor%20Remainder)) (Math|Vector|MakeVector 0.0 (* (Variables|RoomSize|GetTileSizeY) _index_3) 0.0) "0,90.000000, 0"))
    ;[1 1 1] Top Wall
    (CallFunction|WallorDoor (== (Math|Integer|%(Integer) _index_3 (Variables|Default|GetDoor%20Every)) (Variables|Default|GetDoor%20Remainder)) (Math|Vector|MakeVector (* (Math|Conversions|ToFloat(Integer) (Variables|RoomSize|GetRoomTilesX)) (Variables|RoomSize|GetTileSizeX)) (* (Variables|RoomSize|GetTileSizeY) (+ (Math|Conversions|ToFloat(Integer) _index_3) 1.0)) 0.0) "0,-90.000000, 0"))
  (for _index_4 (range 0 (- (Variables|RoomSize|GetRoomTilesX) 1))
    ;[1 1 1] Right Wall
    (CallFunction|WallorDoor (== (Math|Integer|%(Integer) _index_4 (Variables|Default|GetDoor%20Every)) (Variables|Default|GetDoor%20Remainder)) (Math|Vector|MakeVector (* (Variables|RoomSize|GetTileSizeX) (Math|Conversions|ToFloat(Integer) _index_4)) (* (Variables|RoomSize|GetTileSizeY) (Math|Conversions|ToFloat(Integer) (Variables|RoomSize|GetRoomTilesY))) 0.0) "0, 0, 0")
    ;[1 1 1] Left Wall
    (CallFunction|WallorDoor (== (Math|Integer|%(Integer) _index_4 (Variables|Default|GetDoor%20Every)) (Variables|Default|GetDoor%20Remainder)) (Math|Vector|MakeVector (* (Variables|RoomSize|GetTileSizeX) (+ (Math|Conversions|ToFloat(Integer) _index_4) 1.0)) 0.0 0.0) "0,180.000000, 0")))

(fn WallorDoor
  (params (Can%20Door :type Boolean) (Instance%20Transform%20Location :type Vector) (Instance%20Transform%20Rotation :type Rotator))
  (bind _returnvalue (Transformation|GetActorTransform))
  (bind _doorcount (Variables|RoomSize|GetDoorCount))
  (if (and Can%20Door (Class|KismetMathLibrary|RandomBoolwithWeightfromStream (/ (Math|Conversions|ToFloat(Integer) _doorcount) (Math|Conversions|ToFloat(Integer) (- _doorcount (Utilities|Array|Length (Variables|RoomSize|GetDoors))))) (Variables|Default|GetRoomStream)))
    (bind _returnvalue_2 (Game|SpawnActorfromClass "/Game/Blueprints/ProceduralGeneration_Rooms/BP_Door.BP_Door_C" (Math|Transform|MakeTransform (Math|Transform|TransformLocation _returnvalue Instance%20Transform%20Location) (Math|Transform|TransformRotation _returnvalue Instance%20Transform%20Rotation) "1.000000,1.000000,1.000000") "Undefined" 0 0 0))
    (Utilities|Array|Add (Variables|RoomSize|GetDoors) _returnvalue_2)
    (else
      (Components|InstancedStaticMesh|AddInstance (Variables|Default|GetWall) (Math|Transform|MakeTransform Instance%20Transform%20Location Instance%20Transform%20Rotation "1.000000,1.000000,1.000000") false))))

(fn UnderConstructionRoom
  ;[1 1 1] Floor generation
  (for _index (range 0 (- (Variables|RoomSize|GetRoomTilesY) 1))
    (for _index_2 (range 0 (- (Variables|RoomSize|GetRoomTilesX) 1))
      (Components|InstancedStaticMesh|AddInstance (Variables|Default|GetFloor) (Math|Transform|MakeTransform (Math|Vector|MakeVector (* (Math|Conversions|ToFloat(Integer) _index_2) (Variables|RoomSize|GetTileSizeX)) (* (Math|Conversions|ToFloat(Integer) (- _index (Variables|Default|GetEntryShift))) (Variables|RoomSize|GetTileSizeY)) 0.0) "0, 0, 0" "1.000000,1.000000,1.000000") false)))
  (if (not (Variables|Default|GetHall))
    (for _index_3 (range 0 (- (Variables|RoomSize|GetRoomTilesY) 1))
      (if (or (Variables|Default|GetOrigin) (!= _index_3 (Variables|Default|GetEntryShift)))
        ;[1 1 1] Bottom Wall
        (CallFunction|WallorDoorReconstruct (== (Math|Integer|%(Integer) _index_3 (Variables|Default|GetDoor%20Every)) (Variables|Default|GetDoor%20Remainder)) (- (Math|Vector|MakeVector 0.0 (* (Variables|RoomSize|GetTileSizeY) _index_3) 0.0) (Math|Vector|MakeVector 0.0 (* (Variables|Default|GetEntryShift) (Variables|RoomSize|GetTileSizeY)) 0.0)) "0, 0, 0"))
      ;[1 1 1] Top Wall
      (CallFunction|WallorDoorReconstruct (== (Math|Integer|%(Integer) _index_3 (Variables|Default|GetDoor%20Every)) (Variables|Default|GetDoor%20Remainder)) (- (Math|Vector|MakeVector (* (Math|Conversions|ToFloat(Integer) (Variables|RoomSize|GetRoomTilesX)) (Variables|RoomSize|GetTileSizeX)) (* (Variables|RoomSize|GetTileSizeY) (+ (Math|Conversions|ToFloat(Integer) _index_3) 1.0)) 0.0) (Math|Vector|MakeVector 0.0 (* (Variables|Default|GetEntryShift) (Variables|RoomSize|GetTileSizeY)) 0.0)) "0, 0, 0")))
  (for _index_4 (range 0 (- (Variables|RoomSize|GetRoomTilesX) 1))
    ;[1 1 1] Right Wall
    (CallFunction|WallorDoorReconstruct (== (Math|Integer|%(Integer) _index_4 (Variables|Default|GetDoor%20Every)) (Variables|Default|GetDoor%20Remainder)) (- (Math|Vector|MakeVector (* (Variables|RoomSize|GetTileSizeX) (Math|Conversions|ToFloat(Integer) _index_4)) (* (Variables|RoomSize|GetTileSizeY) (Math|Conversions|ToFloat(Integer) (Variables|RoomSize|GetRoomTilesY))) 0.0) (Math|Vector|MakeVector 0.0 (* (Variables|Default|GetEntryShift) (Variables|RoomSize|GetTileSizeY)) 0.0)) "0, 0, 0")
    ;[1 1 1] Left Wall
    (CallFunction|WallorDoorReconstruct (== (Math|Integer|%(Integer) _index_4 (Variables|Default|GetDoor%20Every)) (Variables|Default|GetDoor%20Remainder)) (- (Math|Vector|MakeVector (* (Variables|RoomSize|GetTileSizeX) (+ (Math|Conversions|ToFloat(Integer) _index_4) 1.0)) 0.0 0.0) (Math|Vector|MakeVector 0.0 (* (Variables|Default|GetEntryShift) (Variables|RoomSize|GetTileSizeY)) 0.0)) "0, 0, 0")))

(fn WallorDoorReconstruct
  (params (Can%20Door :type Boolean) (Instance%20Transform%20Location :type Vector) (Instance%20Transform%20Rotation :type Rotator))
  (bind _returnvalue (Transformation|GetActorTransform))
  (bind _doorcount (Variables|RoomSize|GetDoorCount))
  (if (and Can%20Door (Class|KismetMathLibrary|RandomBoolwithWeightfromStream (/ (Math|Conversions|ToFloat(Integer) _doorcount) (Math|Conversions|ToFloat(Integer) (- _doorcount (Utilities|Array|Length (Variables|RoomSize|GetDoors))))) (Variables|Default|GetRoomStream)))
    (bind _returnvalue_2 (Game|SpawnActorfromClass "/Game/Blueprints/ProceduralGeneration_Rooms/BP_Door.BP_Door_C" (Math|Transform|MakeTransform (Math|Transform|TransformLocation _returnvalue Instance%20Transform%20Location) (Math|Transform|TransformRotation _returnvalue Instance%20Transform%20Rotation) "1.000000,1.000000,1.000000") "Undefined" 0 (Class|KismetMathLibrary|RandomIntegerfromStream 10000 (Variables|Default|GetRoomStream)) 0))
    (Utilities|Array|Add (Variables|RoomSize|GetDoors) _returnvalue_2)
    (else
      (Components|InstancedStaticMesh|AddInstance (Variables|Default|GetWall_H) (Math|Transform|MakeTransform Instance%20Transform%20Location Instance%20Transform%20Rotation "1.000000,1.000000,1.000000") false))))