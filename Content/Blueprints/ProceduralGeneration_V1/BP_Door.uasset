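; Interactable door for procedural level generation that swings on a timeline and can spawn a new BP_Room when first opened.
; A seeded stream picks a tile limit, then AddAddition line-traces along the door's right vector for that length.
; Only door or wall-collision hits spawn a room, with X size from hit distance, after disabling that door's Roomify or calling the wall's RemoveIndex.
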(event Custom|NewRoom
  (params (Room%20Tiles%20X :type Integer) (Room%20Tiles%20Y :type Integer) (Shift :type Integer) (Max%20Doors :type Integer) (Hall :type Boolean))
  (Game|SpawnActorfromClass "/Game/Blueprints/ProceduralGeneration_V1/BP_Room.BP_Room_C" (Math|Transform|MakeTransform (+ (Transformation|GetActorLocation) (* (Transformation|GetActorForwardVector) 4e+02)) (Math|Rotator|CombineRotators (Transformation|GetActorRotation) "0,90.000000, 0") "1.000000,1.000000,1.000000") "Undefined" 0 Room%20Tiles%20X Room%20Tiles%20Y Max%20Doors Hall Shift 0))

(event Custom|AddAddition
  (bind _returnvalue (Transformation|GetActorTransform))
  (bind _returnvalue_2 (Math|Transform|TransformLocation _returnvalue "0, 0, 0"))
  (bind (_outhit _returnvalue_3) (Collision|LineTraceByChannel _returnvalue_2 (+ _returnvalue_2 (* (Transformation|GetActorRightVector) (* (Variables|Default|GetRoomSizeLimit) (Variables|Default|GetTileSize)))) "TraceTypeQuery1" false 0 "Persistent"))
  (if _returnvalue_3
    (switch string (Utilities|GetClassDisplayName (Utilities|GetClass (.HitActor (Collision|BreakHitResult _outhit))))
      (:BP_Door_C
        (bind _asbp_door (Utilities|Casting|CastToBP_Door (.HitActor (Collision|BreakHitResult _outhit))))
        (Variables|BP_Door_C|SetRoomify _asbp_door false))
      (:BP_WallCollision_C
        (bind _asbp_wall_collision (Utilities|Casting|CastToBP_WallCollision (.HitActor (Collision|BreakHitResult _outhit))))
        (Default|RemoveIndex _asbp_wall_collision)))
    (CallFunction|NewRoom (Math|Float|Round (/ (.Distance (Collision|BreakHitResult _outhit)) (Variables|Default|GetTileSize))) 0 0 (Math|Random|RandomIntegerinRangefromStream 0 2 (Variables|Default|GetDoorStream)) false)))

(event EventInteractDoor
  (if (Variables|Default|GetIsDoorClosed)
    (Variables|Default|SetIsDoorClosed false)
    (Utilities|FlowControl|Sequence
      (:then_0
        (Utilities|FlowControl|DoOnce (Variables|Default|GetRoomify)
          (:Completed
            (Variables|Default|SetRoomify false)
            (bind _output_get (Variables|Default|SetRoomSizeLimit (Math|Random|RandomIntegerinRangefromStream 3 10 (Variables|Default|GetDoorStream))))
            (bind _output_get_2 (Variables|Default|SetLeftLimit _output_get))
            (Variables|Default|SetRightLimit _output_get_2)
            (CallFunction|AddAddition))))
      (:then_1
        (bind _dooryaw (Timeline|OpenDoor Play)
          (:Update
            (Transformation|SetRelativeRotation (Variables|Default|GetDoorHinge) (Math|Rotator|MakeRotator 0.0 0.0 _dooryaw) false false)))))
    (else
      (Variables|Default|SetIsDoorClosed true)
      (Timeline|OpenDoor Reverse))))

(event EventBeginPlay
  (Variables|Default|SetDoorStream (Math|Random|MakeRandomStream (Variables|Default|GetSeed))))

(fn ConstructionScript)

(fn InteractLoadout
  (params (Interactor :type BP%20Player%20Object%20Reference))
  (return false))