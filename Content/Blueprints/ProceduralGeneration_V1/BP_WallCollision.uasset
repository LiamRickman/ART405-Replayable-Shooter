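; BP_WallCollision is a procedural generation actor that stands for one indexed wall of a room.
; On BeginPlay it runs Update, which stores the index and shows it on a text render component.
; RemoveIndex tells the owning Room to remove the wall at that index, then destroys the actor.
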(event Custom|Update
  (params (Index :type Integer))
  (bind _output_get (Variables|Default|SetIndex Index))
  (Rendering|Components|TextRender|SetText (Variables|Default|GetTextRender) (Utilities|Text|ToText(Integer) _output_get)))

(event Custom|RemoveIndex
  (Default|RemoveWall (Variables|Default|GetRoom) (Variables|Default|GetIndex))
  (Actor|DestroyActor))

(event EventBeginPlay
  (CallFunction|Update (Variables|Default|GetIndex)))

(fn ConstructionScript)