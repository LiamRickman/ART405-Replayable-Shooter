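; Legacy parent Blueprint for procedurally generated level rooms, kept in an Old folder.
; On BeginPlay it gathers its twelve wall references into WallArray.
; CalculateDoors takes a room direction plus start and end doors but is an empty stub here, and the construction script is also empty.
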(event Custom|CalculateDoors
  (params (RoomDirection :type String) (StartDoor :type Integer) (EndDoor :type Integer)))

(event EventBeginPlay
  (Variables|Default|SetWallArray (Utilities|Array|MakeArray (Variables|Default|GetWall1) (Variables|Default|GetWall2) (Variables|Default|GetWall3) (Variables|Default|GetWall4) (Variables|Default|GetWall5) (Variables|Default|GetWall6) (Variables|Default|GetWall7) (Variables|Default|GetWall8) (Variables|Default|GetWall9) (Variables|Default|GetWall10) (Variables|Default|GetWall11) (Variables|Default|GetWall12))))

(fn ConstructionScript)