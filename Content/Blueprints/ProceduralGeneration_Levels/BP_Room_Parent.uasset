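; Parent room actor for procedural level generation, with three wall segments per side, any of which can hold that side's door.
; BeginPlay builds the wall arrays and randomly picks a door slot for each side.
; GenerateDoors tags the chosen segment on active sides, then UpdateWalls swaps every segment's mesh by its IsDoor tag.
; Helpers remap doors for quarter-turn rotations and destroy the room if it has no hallways.
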(event Custom|UpdateWalls
  (for _array_element (Variables|Default|GetWallArray)
    (if (Components|ComponentHasTag _array_element "IsDoor")
      (Components|StaticMesh|SetStaticMesh _array_element "/Game/StarterContent/Architecture/Wall_Door_400x400.Wall_Door_400x400")
      (else
        (Components|StaticMesh|SetStaticMesh _array_element "/Game/StarterContent/Architecture/Wall_400x400.Wall_400x400")))))

(event Custom|GenerateDoors
  (CallFunction|SetFrontDoor)
  (CallFunction|SetRightDoor)
  (CallFunction|SetBackDoor)
  (CallFunction|SetLeftDoor)
  (CallFunction|UpdateWalls))

(event Custom|DeleteIfNoHallway
  (if (< (Variables|Default|GetHallways) 1)
    (Actor|DestroyActor)))

(event EventBeginPlay
  (CallFunction|SetWallArrays)
  (CallFunction|GetRandomDoors))

(fn ConstructionScript)

(fn SetWallArrays
  (Variables|Default|SetFrontWallArray (Utilities|Array|MakeArray (Variables|Default|GetWall_Front_1) (Variables|Default|GetWall_Front_2) (Variables|Default|GetWall_Front_3)))
  (Variables|Default|SetRightWallArray (Utilities|Array|MakeArray (Variables|Default|GetWall_Right_1) (Variables|Default|GetWall_Right_2) (Variables|Default|GetWall_Right_3)))
  (Variables|Default|SetBackWallArray (Utilities|Array|MakeArray (Variables|Default|GetWall_Back_1) (Variables|Default|GetWall_Back_2) (Variables|Default|GetWall_Back_3)))
  (Variables|Default|SetLeftWallArray (Utilities|Array|MakeArray (Variables|Default|GetWall_Left_1) (Variables|Default|GetWall_Left_2) (Variables|Default|GetWall_Left_3)))
  (Utilities|Array|Clear (Variables|Default|GetWallArray))
  (for _array_element (Variables|Default|GetFrontWallArray)
    (Utilities|Array|Add (Variables|Default|GetWallArray) _array_element))
  (for _array_element_2 (Variables|Default|GetRightWallArray)
    (Utilities|Array|Add (Variables|Default|GetWallArray) _array_element_2))
  (for _array_element_3 (Variables|Default|GetBackWallArray)
    (Utilities|Array|Add (Variables|Default|GetWallArray) _array_element_3))
  (for _array_element_4 (Variables|Default|GetLeftWallArray)
    (Utilities|Array|Add (Variables|Default|GetWallArray) _array_element_4)))

(fn SetRandomDoors
  (bind _rightwallarray (Variables|Default|GetRightWallArray))
  (bind _backwallarray (Variables|Default|GetBackWallArray))
  (bind _leftwallarray (Variables|Default|GetLeftWallArray))
  (bind _frontwallarray (Variables|Default|GetFrontWallArray))
  (for _array_element _frontwallarray
    (Variables|/Script/Engine.ActorComponent|SetComponentTags _array_element (LocalVariables|GetTags_FrontWall)))
  (Variables|/Script/Engine.ActorComponent|SetComponentTags (Utilities|Array|Get(acopy) _frontwallarray (Math|Random|RandomIntegerinRange 0 (- (Utilities|Array|Length _frontwallarray) 1))) (LocalVariables|GetTags_FrontWall_Door))
  (for _array_element_2 _rightwallarray
    (Variables|/Script/Engine.ActorComponent|SetComponentTags _array_element_2 (LocalVariables|GetTags_RightWall)))
  (Variables|/Script/Engine.ActorComponent|SetComponentTags (Utilities|Array|Get(acopy) _rightwallarray (Math|Random|RandomIntegerinRange 0 (- (Utilities|Array|Length _rightwallarray) 1))) (LocalVariables|GetTags_RightWall_Door))
  (for _array_element_3 _backwallarray
    (Variables|/Script/Engine.ActorComponent|SetComponentTags _array_element_3 (LocalVariables|GetTags_BackWall)))
  (Variables|/Script/Engine.ActorComponent|SetComponentTags (Utilities|Array|Get(acopy) _backwallarray (Math|Random|RandomIntegerinRange 0 (- (Utilities|Array|Length _backwallarray) 1))) (LocalVariables|GetTags_BackWall_Door))
  (for _array_element_4 _leftwallarray
    (Variables|/Script/Engine.ActorComponent|SetComponentTags _array_element_4 (LocalVariables|GetTags_LeftWall)))
  (Variables|/Script/Engine.ActorComponent|SetComponentTags (Utilities|Array|Get(acopy) _leftwallarray (Math|Random|RandomIntegerinRange 0 (- (Utilities|Array|Length _leftwallarray) 1))) (LocalVariables|GetTags_LeftWall_Door)))

(fn SetDoor
  (params (Door%20# :type Integer) (WallDir :type String))
  (Utilities|Array|Clear (LocalVariables|GetWallsToCheck))
  (switch string WallDir
    (:Front
      (LocalVariables|SetWallsToCheck (Variables|Default|GetFrontWallArray))
      (LocalVariables|SetDoorTagsToUse (LocalVariables|GetTags_FrontWall_Door))
      (LocalVariables|SetWallTagsToUse (LocalVariables|GetTags_FrontWall)))
    (:Right
      (LocalVariables|SetWallsToCheck (Variables|Default|GetRightWallArray))
      (LocalVariables|SetDoorTagsToUse (LocalVariables|GetTags_RightWall_Door))
      (LocalVariables|SetWallTagsToUse (LocalVariables|GetTags_RightWall)))
    (:Back
      (LocalVariables|SetWallsToCheck (Variables|Default|GetBackWallArray))
      (LocalVariables|SetDoorTagsToUse (LocalVariables|GetTags_BackWall_Door))
      (LocalVariables|SetWallTagsToUse (LocalVariables|GetTags_BackWall)))
    (:Left
      (LocalVariables|SetWallsToCheck (Variables|Default|GetLeftWallArray))
      (LocalVariables|SetDoorTagsToUse (LocalVariables|GetTags_LeftWall_Door))
      (LocalVariables|SetWallTagsToUse (LocalVariables|GetTags_LeftWall))))
  (for _array_element (LocalVariables|GetWallsToCheck)
    (Variables|/Script/Engine.ActorComponent|SetComponentTags _array_element (LocalVariables|GetWallTagsToUse)))
  (Variables|/Script/Engine.ActorComponent|SetComponentTags (Utilities|Array|Get(acopy) (LocalVariables|GetWallsToCheck) (- Door%20# 1)) (LocalVariables|GetDoorTagsToUse)))

(fn SetFrontDoor
  (if (Variables|Default|GetFrontDoorActive)
    (switch int (Variables|Default|GetFrontDoor)
      (:1
        (Variables|/Script/Engine.ActorComponent|SetComponentTags (Variables|Default|GetWall_Front_1) (LocalVariables|GetDoorTags))
        (Variables|/Script/Engine.ActorComponent|SetComponentTags (Variables|Default|GetWall_Front_2) (LocalVariables|GetWallTags))
        (Variables|/Script/Engine.ActorComponent|SetComponentTags (Variables|Default|GetWall_Front_3) (LocalVariables|GetWallTags)))
      (:2
        (Variables|/Script/Engine.ActorComponent|SetComponentTags (Variables|Default|GetWall_Front_2) (LocalVariables|GetDoorTags))
        (Variables|/Script/Engine.ActorComponent|SetComponentTags (Variables|Default|GetWall_Front_1) (LocalVariables|GetWallTags))
        (Variables|/Script/Engine.ActorComponent|SetComponentTags (Variables|Default|GetWall_Front_3) (LocalVariables|GetWallTags)))
      (:3
        (Variables|/Script/Engine.ActorComponent|SetComponentTags (Variables|Default|GetWall_Front_3) (LocalVariables|GetDoorTags))
        (Variables|/Script/Engine.ActorComponent|SetComponentTags (Variables|Default|GetWall_Front_1) (LocalVariables|GetWallTags))
        (Variables|/Script/Engine.ActorComponent|SetComponentTags (Variables|Default|GetWall_Front_2) (LocalVariables|GetWallTags))))
    (return)
    (else
      (return))))

(fn SetRightDoor
  (if (Variables|Default|GetRightDoorActive)
    (switch int (Variables|Default|GetRightDoor)
      (:1
        (Variables|/Script/Engine.ActorComponent|SetComponentTags (Variables|Default|GetWall_Right_1) (LocalVariables|GetDoorTags))
        (Variables|/Script/Engine.ActorComponent|SetComponentTags (Variables|Default|GetWall_Right_2) (LocalVariables|GetWallTags))
        (Variables|/Script/Engine.ActorComponent|SetComponentTags (Variables|Default|GetWall_Right_3) (LocalVariables|GetWallTags)))
      (:2
        (Variables|/Script/Engine.ActorComponent|SetComponentTags (Variables|Default|GetWall_Right_2) (LocalVariables|GetDoorTags))
        (Variables|/Script/Engine.ActorComponent|SetComponentTags (Variables|Default|GetWall_Right_1) (LocalVariables|GetWallTags))
        (Variables|/Script/Engine.ActorComponent|SetComponentTags (Variables|Default|GetWall_Right_3) (LocalVariables|GetWallTags)))
      (:3
        (Variables|/Script/Engine.ActorComponent|SetComponentTags (Variables|Default|GetWall_Right_3) (LocalVariables|GetDoorTags))
        (Variables|/Script/Engine.ActorComponent|SetComponentTags (Variables|Default|GetWall_Right_1) (LocalVariables|GetWallTags))
        (Variables|/Script/Engine.ActorComponent|SetComponentTags (Variables|Default|GetWall_Right_2) (LocalVariables|GetWallTags))))
    (return)
    (else
      (return))))

(fn SetBackDoor
  (if (Variables|Default|GetBackDoorActive)
    (switch int (Variables|Default|GetBackDoor)
      (:1
        (Variables|/Script/Engine.ActorComponent|SetComponentTags (Variables|Default|GetWall_Back_1) (LocalVariables|GetDoorTags))
        (Variables|/Script/Engine.ActorComponent|SetComponentTags (Variables|Default|GetWall_Back_2) (LocalVariables|GetWallTags))
        (Variables|/Script/Engine.ActorComponent|SetComponentTags (Variables|Default|GetWall_Back_3) (LocalVariables|GetWallTags)))
      (:2
        (Variables|/Script/Engine.ActorComponent|SetComponentTags (Variables|Default|GetWall_Back_2) (LocalVariables|GetDoorTags))
        (Variables|/Script/Engine.ActorComponent|SetComponentTags (Variables|Default|GetWall_Back_1) (LocalVariables|GetWallTags))
        (Variables|/Script/Engine.ActorComponent|SetComponentTags (Variables|Default|GetWall_Back_3) (LocalVariables|GetWallTags)))
      (:3
        (Variables|/Script/Engine.ActorComponent|SetComponentTags (Variables|Default|GetWall_Back_3) (LocalVariables|GetDoorTags))
        (Variables|/Script/Engine.ActorComponent|SetComponentTags (Variables|Default|GetWall_Back_1) (LocalVariables|GetWallTags))
        (Variables|/Script/Engine.ActorComponent|SetComponentTags (Variables|Default|GetWall_Back_2) (LocalVariables|GetWallTags))))
    (return)
    (else
      (return))))

(fn SetLeftDoor
  (if (Variables|Default|GetLeftDoorActive)
    (switch int (Variables|Default|GetLeftDoor)
      (:1
        (Variables|/Script/Engine.ActorComponent|SetComponentTags (Variables|Default|GetWall_Left_1) (LocalVariables|GetDoorTags))
        (Variables|/Script/Engine.ActorComponent|SetComponentTags (Variables|Default|GetWall_Left_2) (LocalVariables|GetWallTags))
        (Variables|/Script/Engine.ActorComponent|SetComponentTags (Variables|Default|GetWall_Left_3) (LocalVariables|GetWallTags)))
      (:2
        (Variables|/Script/Engine.ActorComponent|SetComponentTags (Variables|Default|GetWall_Left_2) (LocalVariables|GetDoorTags))
        (Variables|/Script/Engine.ActorComponent|SetComponentTags (Variables|Default|GetWall_Left_1) (LocalVariables|GetWallTags))
        (Variables|/Script/Engine.ActorComponent|SetComponentTags (Variables|Default|GetWall_Left_3) (LocalVariables|GetWallTags)))
      (:3
        (Variables|/Script/Engine.ActorComponent|SetComponentTags (Variables|Default|GetWall_Left_3) (LocalVariables|GetDoorTags))
        (Variables|/Script/Engine.ActorComponent|SetComponentTags (Variables|Default|GetWall_Left_1) (LocalVariables|GetWallTags))
        (Variables|/Script/Engine.ActorComponent|SetComponentTags (Variables|Default|GetWall_Left_2) (LocalVariables|GetWallTags))))
    (return)
    (else
      (return))))

(fn GetRandomDoors
  (Variables|Default|SetFrontDoor (Math|Random|RandomIntegerinRange 1 3))
  (Variables|Default|SetRightDoor (Math|Random|RandomIntegerinRange 1 3))
  (Variables|Default|SetBackDoor (Math|Random|RandomIntegerinRange 1 3))
  (Variables|Default|SetLeftDoor (Math|Random|RandomIntegerinRange 1 3)))

(fn GetRotatedDoors
  (params (Rotation :type Integer))
  (bind _output_get (Variables|Default|SetCurrentRotation Rotation))
  (switch int _output_get
    (:0
      (return (Variables|Default|GetFrontDoor) (Variables|Default|GetRightDoor) (Variables|Default|GetBackDoor) (Variables|Default|GetLeftDoor) (Variables|Default|GetFrontDoorActive) (Variables|Default|GetRightDoorActive) (Variables|Default|GetBackDoorActive) (Variables|Default|GetLeftDoorActive)))
    (:1
      (return (Variables|Default|GetRightDoor) (Variables|Default|GetBackDoor) (Variables|Default|GetLeftDoor) (Variables|Default|GetFrontDoor) (Variables|Default|GetRightDoorActive) (Variables|Default|GetBackDoorActive) (Variables|Default|GetLeftDoorActive) (Variables|Default|GetFrontDoorActive)))
    (:2
      (return (Variables|Default|GetBackDoor) (Variables|Default|GetLeftDoor) (Variables|Default|GetFrontDoor) (Variables|Default|GetRightDoor) (Variables|Default|GetBackDoorActive) (Variables|Default|GetLeftDoorActive) (Variables|Default|GetFrontDoorActive) (Variables|Default|GetRightDoorActive)))
    (:3
      (return (Variables|Default|GetLeftDoor) (Variables|Default|GetFrontDoor) (Variables|Default|GetRightDoor) (Variables|Default|GetBackDoor) (Variables|Default|GetLeftDoorActive) (Variables|Default|GetFrontDoorActive) (Variables|Default|GetRightDoorActive) (Variables|Default|GetBackDoorActive)))))

(fn SetRotatedDoors
  (params (RotatedFrontDoor :type Integer) (RotatedRightDoor :type Integer) (RotatedBackDoor :type Integer) (RotatedLeftDoor :type Integer) (RotatedFrontDoorActive :type Boolean) (RotatedRightDoorActive :type Boolean) (RotatedBackDoorActive :type Boolean) (RotatedLeftDoorActive :type Boolean))
  (Variables|Default|SetFrontDoor RotatedFrontDoor)
  (Variables|Default|SetRightDoor RotatedRightDoor)
  (Variables|Default|SetBackDoor RotatedBackDoor)
  (Variables|Default|SetLeftDoor RotatedLeftDoor)
  (Variables|Default|SetFrontDoorActive RotatedFrontDoorActive)
  (Variables|Default|SetRightDoorActive RotatedRightDoorActive)
  (Variables|Default|SetBackDoorActive RotatedBackDoorActive)
  (Variables|Default|SetLeftDoorActive RotatedLeftDoorActive)
  (CallFunction|GenerateDoors))