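; Procedural level generator that, on BeginPlay, lays out a random walk of NumberOfRooms generic rooms joined by hallways.
; Each step avoids reversing LastRoom's direction, but has no overlap check.
; Spawn functions pick random start/end doors, select a matching hallway variant, then offset CurrentRoomPos by tile size.
; RandomInteger's exclusive max leaves each switch's last case unreachable, so Right rooms never spawn.
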(event EventBeginPlay
  (for _index (range 1 (Variables|Default|GetNumberOfRooms))
    (if (Variables|Default|GetIsFirstRoom)
      (switch int (Math|Random|RandomInteger 1)
        (:0
          (CallFunction|SpawnFrontRoom))
        (:1
          (CallFunction|SpawnBackRoom)))
      (else
        (switch string (Variables|Default|GetLastRoom)
          (:Front
            (switch int (Math|Random|RandomInteger 2)
              (:0
                (CallFunction|SpawnFrontRoom))
              (:1
                (CallFunction|SpawnLeftRoom))
              (:2
                (CallFunction|SpawnRightRoom))))
          (:Back
            (switch int (Math|Random|RandomInteger 2)
              (:0
                (CallFunction|SpawnBackRoom))
              (:1
                (CallFunction|SpawnLeftRoom))
              (:2
                (CallFunction|SpawnRightRoom))))
          (:Left
            (switch int (Math|Random|RandomInteger 2)
              (:0
                (CallFunction|SpawnFrontRoom))
              (:1
                (CallFunction|SpawnBackRoom))
              (:2
                (CallFunction|SpawnRightRoom))))
          (:Right
            (switch int (Math|Random|RandomInteger 2)
              (:0
                (CallFunction|SpawnFrontRoom))
              (:1
                (CallFunction|SpawnLeftRoom))
              (:2
                (CallFunction|SpawnBackRoom)))))))))

(fn ConstructionScript)

(fn SpawnFrontRoom
  (if (Variables|Default|GetIsFirstRoom)
    (LocalVariables|SetStartDoor 2)
    (Variables|Default|SetIsFirstRoom false)
    (else
      (LocalVariables|SetStartDoor (Math|Random|RandomIntegerinRange 1 3))))
  (LocalVariables|SetEndDoor (Math|Random|RandomIntegerinRange 1 3))
  (CallFunction|CalculateHallwayType (LocalVariables|GetStartDoor) (LocalVariables|GetEndDoor))
  (Variables|Default|SetHallwaySpawnPos (+ (Variables|Default|GetCurrentRoomPos) (Math|Vector|MakeVector (* (Variables|Default|GetTileSize) 3.0) (* (Variables|Default|GetTileSize) (- (LocalVariables|GetStartDoor) 1)) 0.0)))
  (bind _output_get (Variables|Default|SetCurrentRoomPos (+ (Variables|Default|GetCurrentRoomPos) (Math|Vector|MakeVector (* (Variables|Default|GetTileSize) (+ (Variables|Default|GetHallwaySize) 3.0)) 0.0 0.0))))
  (Game|SpawnActorfromClass "/Game/Blueprints/ProceduralGeneration_Levels/Old/BP_Room_Generic_OLD.BP_Room_Generic_OLD_C" (Math|Transform|MakeTransform _output_get "0, 0, 0" "1.000000,1.000000,1.000000") "Undefined" 0 0)
  (Game|SpawnActorfromClass (Variables|Default|GetHallwayType) (Math|Transform|MakeTransform (Variables|Default|GetHallwaySpawnPos) "0, 0, 0" "1.000000,1.000000,1.000000") "Undefined" 0 0)
  (Variables|Default|SetLastRoom "Front"))

(fn CalculateHallwayType
  (params (StartDoor :type Integer) (EndDoor :type Integer))
  (if (== StartDoor EndDoor)
    (Variables|Default|SetHallwayType "/Game/Blueprints/ProceduralGeneration_Levels/Hallways/BP_Hallway_V1.BP_Hallway_V1_C")
    (elif (or (and (== StartDoor 1) (== EndDoor 2)) (and (== StartDoor 2) (== EndDoor 3)))
      (Variables|Default|SetHallwayType "/Game/Blueprints/ProceduralGeneration_Levels/Hallways/BP_Hallway_V2.BP_Hallway_V2_C")
      (elif (and (== StartDoor 1) (== EndDoor 3))
        (Variables|Default|SetHallwayType "/Game/Blueprints/ProceduralGeneration_Levels/Hallways/BP_Hallway_V3.BP_Hallway_V3_C")
        (elif (or (and (== StartDoor 2) (== EndDoor 1)) (and (== StartDoor 3) (== EndDoor 2)))
          (Variables|Default|SetHallwayType "/Game/Blueprints/ProceduralGeneration_Levels/Hallways/BP_Hallway_V4.BP_Hallway_V4_C")
          (elif (and (== StartDoor 3) (== EndDoor 1))
            (Variables|Default|SetHallwayType "/Game/Blueprints/ProceduralGeneration_Levels/Hallways/BP_Hallway_V5.BP_Hallway_V5_C")
            (else
              (Development|PrintString "Appropriate Hallway Not Found!"))))))))

(fn SpawnRightRoom
  (bind _tilesize (Variables|Default|GetTileSize))
  (bind _returnvalue (* _tilesize 3.0))
  (if (Variables|Default|GetIsFirstRoom)
    (LocalVariables|SetStartDoor 2)
    (Variables|Default|SetIsFirstRoom false)
    (else
      (LocalVariables|SetStartDoor (Math|Random|RandomIntegerinRange 1 3))))
  (LocalVariables|SetEndDoor (Math|Random|RandomIntegerinRange 1 3))
  (CallFunction|CalculateHallwayType (LocalVariables|GetStartDoor) (LocalVariables|GetEndDoor))
  (Variables|Default|SetHallwaySpawnPos (+ (Variables|Default|GetCurrentRoomPos) (Math|Vector|MakeVector (+ _returnvalue (* (Variables|Default|GetTileSize) (* (- (LocalVariables|GetStartDoor) 1) -1))) _returnvalue 0.0)))
  (bind _output_get (Variables|Default|SetCurrentRoomPos (+ (Variables|Default|GetCurrentRoomPos) (Math|Vector|MakeVector 0.0 (* (Variables|Default|GetTileSize) (+ (Variables|Default|GetHallwaySize) 3.0)) 0.0))))
  (Game|SpawnActorfromClass "/Game/Blueprints/ProceduralGeneration_Levels/Old/BP_Room_Generic_OLD.BP_Room_Generic_OLD_C" (Math|Transform|MakeTransform _output_get "0, 0, 0" "1.000000,1.000000,1.000000") "Undefined" 0 0)
  (Game|SpawnActorfromClass (Variables|Default|GetHallwayType) (Math|Transform|MakeTransform (Variables|Default|GetHallwaySpawnPos) "0,90.000000, 0" "1.000000,1.000000,1.000000") "Undefined" 0 0)
  (Variables|Default|SetLastRoom "Right"))

(fn SpawnLeftRoom
  (if (Variables|Default|GetIsFirstRoom)
    (LocalVariables|SetStartDoor 2)
    (Variables|Default|SetIsFirstRoom false)
    (else
      (LocalVariables|SetStartDoor (Math|Random|RandomIntegerinRange 1 3))))
  (LocalVariables|SetEndDoor (Math|Random|RandomIntegerinRange 1 3))
  (CallFunction|CalculateHallwayType (LocalVariables|GetStartDoor) (LocalVariables|GetEndDoor))
  (Variables|Default|SetHallwaySpawnPos (+ (Variables|Default|GetCurrentRoomPos) (Math|Vector|MakeVector (* (Variables|Default|GetTileSize) (- (LocalVariables|GetStartDoor) 1)) 0.0 0.0)))
  (bind _output_get (Variables|Default|SetCurrentRoomPos (+ (Variables|Default|GetCurrentRoomPos) (Math|Vector|MakeVector 0.0 (* (* (Variables|Default|GetTileSize) (+ (Variables|Default|GetHallwaySize) 3.0)) -1.0) 0.0))))
  (Game|SpawnActorfromClass "/Game/Blueprints/ProceduralGeneration_Levels/Old/BP_Room_Generic_OLD.BP_Room_Generic_OLD_C" (Math|Transform|MakeTransform _output_get "0, 0, 0" "1.000000,1.000000,1.000000") "Undefined" 0 0)
  (Game|SpawnActorfromClass (Variables|Default|GetHallwayType) (Math|Transform|MakeTransform (Variables|Default|GetHallwaySpawnPos) "0,-90.000000, 0" "1.000000,1.000000,1.000000") "Undefined" 0 0)
  (Variables|Default|SetLastRoom "Left"))

(fn SpawnBackRoom
  (if (Variables|Default|GetIsFirstRoom)
    (LocalVariables|SetStartDoor 2)
    (Variables|Default|SetIsFirstRoom false)
    (else
      (LocalVariables|SetStartDoor (Math|Random|RandomIntegerinRange 1 3))))
  (LocalVariables|SetEndDoor (Math|Random|RandomIntegerinRange 1 3))
  (CallFunction|CalculateHallwayType (LocalVariables|GetStartDoor) (LocalVariables|GetEndDoor))
  (Variables|Default|SetHallwaySpawnPos (+ (Variables|Default|GetCurrentRoomPos) (Math|Vector|MakeVector 0.0 (+ (* (Variables|Default|GetTileSize) 3.0) (* (* (Variables|Default|GetTileSize) (- (LocalVariables|GetStartDoor) 1)) -1.0)) 0.0)))
  (bind _output_get (Variables|Default|SetCurrentRoomPos (+ (Variables|Default|GetCurrentRoomPos) (Math|Vector|MakeVector (* (* (Variables|Default|GetTileSize) (+ (Variables|Default|GetHallwaySize) 3.0)) -1.0) 0.0 0.0))))
  (Game|SpawnActorfromClass "/Game/Blueprints/ProceduralGeneration_Levels/Old/BP_Room_Generic_OLD.BP_Room_Generic_OLD_C" (Math|Transform|MakeTransform _output_get "0, 0, 0" "1.000000,1.000000,1.000000") "Undefined" 0 0)
  (Game|SpawnActorfromClass (Variables|Default|GetHallwayType) (Math|Transform|MakeTransform (Variables|Default|GetHallwaySpawnPos) "0,180.000000, 0" "1.000000,1.000000,1.000000") "Undefined" 0 0)
  (Variables|Default|SetLastRoom "Back"))