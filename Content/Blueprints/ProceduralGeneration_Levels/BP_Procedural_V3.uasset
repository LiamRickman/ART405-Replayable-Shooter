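; Procedural level generator that lays out a grid of rooms on BeginPlay.
; It snakes column by column from a random start direction, spawning BP_Room_Parent placeholders with random rotation and height offset.
; It then shuffles and deletes some rooms for gaps, and swaps others for BP_Room_V1–V3 within per-type counts.
; Hallway types are chosen but not spawned during generation, and the spawn-move step is disconnected.
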(event EventBeginPlay
  (bind _gridsizey (Variables|Grid|GetGridSizeY))
  (Input|EnableInput (Game|GetPlayerController 0))
  (if (== (Math|Random|RandomIntegerinRange 0 1) 0)
    (for _index (range 2 _gridsizey)
      (CallFunction|SpawnFrontRoom))
    (Variables|Grid|SetGridAtTop true)
    (else
      (for _index_2 (range 2 _gridsizey)
        (CallFunction|SpawnBackRoom))
      (Variables|Grid|SetGridAtTop false)))
  (for _index_3 (range 2 (Variables|Grid|GetGridSizeX))
    (CallFunction|SpawnLeftRoom)
    (for _index_4 (range 2 (Variables|Grid|GetGridSizeY))
      (if (Variables|Grid|GetGridAtTop)
        (CallFunction|SpawnBackRoom)
        (else
          (CallFunction|SpawnFrontRoom))))
    (if (Utilities|Enum|Equal(Enum) (Variables|Default|GetLastRoomDirection) "Front")
      (Variables|Grid|SetGridAtTop true)
      (else
        (Variables|Grid|SetGridAtTop false))))
  (CallFunction|DeleteRooms)
  (CallFunction|ReplaceRooms))

(fn ConstructionScript
  (Variables|RoomStats|SetTotalRooms (- (* (Variables|Grid|GetGridSizeX) (Variables|Grid|GetGridSizeY)) 1))
  (Variables|RoomStats|SetExtraRooms (+ (Variables|RoomTypes|GetNumOfRoom1) (Variables|RoomTypes|GetNumOfRoom2) (Variables|RoomTypes|GetNumOfRoom3)))
  (Variables|RoomStats|SetDeletedAndExtraRooms (+ (Variables|RoomStats|GetDeletedRooms) (Variables|RoomStats|GetExtraRooms))))

(fn SpawnFrontRoom
  (bind _tilesize (Variables|Default|GetTileSize))
  (if (Variables|Default|GetIsFirstRoom)
    (LocalVariables|SetStartDoor 2)
    (Variables|Default|SetIsFirstRoom false)
    (else
      (LocalVariables|SetStartDoor (Math|Random|RandomIntegerinRange 1 3))))
  (LocalVariables|SetEndDoor (Math|Random|RandomIntegerinRange 1 3))
  (CallFunction|PickHallwayType (LocalVariables|GetStartDoor) (LocalVariables|GetEndDoor))
  (bind _roomtype (CallFunction|PickRoomType))
  (Variables|Default|SetRoomType _roomtype)
  (Variables|Default|SetHallwaySpawnPos (+ (Variables|Default|GetCurrentRoomPos) (Math|Vector|MakeVector (* (Variables|Default|GetTileSize) 1.5) (+ (* _tilesize -0.5) (* _tilesize (- (LocalVariables|GetStartDoor) 2))) 0.0)))
  (bind _output_get (Variables|Default|SetCurrentRoomPos (+ (Math|Vector|MakeVector (.x (Variables|Default|GetCurrentRoomPos)) (.y (Variables|Default|GetCurrentRoomPos)) 0.0) (Math|Vector|MakeVector (* (Variables|Default|GetTileSize) (+ (Variables|Default|GetHallwaySize) 3.0)) 0.0 (/ (* (Variables|Grid|GetHeightOffset) (Math|Random|RandomIntegerinRange -1 1)) (Math|Random|RandomIntegerinRange 1 2))))))
  (switch int (Math|Random|RandomIntegerinRange 0 3)
    (:0
      (LocalVariables|SetRoomRotation "0, 0, 0"))
    (:1
      (LocalVariables|SetRoomRotation "0,90.000000, 0"))
    (:2
      (LocalVariables|SetRoomRotation "0,180.000000, 0"))
    (:3
      (LocalVariables|SetRoomRotation "0,270.000000, 0")))
  (Game|SpawnActorfromClass (Variables|Default|GetRoomType) (Math|Transform|MakeTransform _output_get (LocalVariables|GetRoomRotation) "1.000000,1.000000,1.000000") "Undefined" 0 0)
  (Variables|Default|SetLastRoomDirection "Front"))

(fn SpawnRightRoom
  (bind _tilesize (Variables|Default|GetTileSize))
  (if (Variables|Default|GetIsFirstRoom)
    (LocalVariables|SetStartDoor 2)
    (Variables|Default|SetIsFirstRoom false)
    (else
      (LocalVariables|SetStartDoor (Math|Random|RandomIntegerinRange 1 3))))
  (LocalVariables|SetEndDoor (Math|Random|RandomIntegerinRange 1 3))
  (CallFunction|PickHallwayType (LocalVariables|GetStartDoor) (LocalVariables|GetEndDoor))
  (Variables|Default|SetHallwaySpawnPos (+ (Variables|Default|GetCurrentRoomPos) (Math|Vector|MakeVector (+ (* _tilesize 0.5) (* _tilesize (* (- (LocalVariables|GetStartDoor) 2) -1))) (* (Variables|Default|GetTileSize) 1.5) 0.0)))
  (bind _output_get (Variables|Default|SetCurrentRoomPos (+ (Math|Vector|MakeVector (.x (Variables|Default|GetCurrentRoomPos)) (.y (Variables|Default|GetCurrentRoomPos)) 0.0) (Math|Vector|MakeVector 0.0 (* (Variables|Default|GetTileSize) (+ (Variables|Default|GetHallwaySize) 3.0)) (/ (* (Variables|Grid|GetHeightOffset) (Math|Random|RandomIntegerinRange -1 1)) (Math|Random|RandomIntegerinRange 1 2))))))
  (switch int (Math|Random|RandomIntegerinRange 0 3)
    (:0
      (LocalVariables|SetRoomRotation "0, 0, 0"))
    (:1
      (LocalVariables|SetRoomRotation "0,90.000000, 0"))
    (:2
      (LocalVariables|SetRoomRotation "0,180.000000, 0"))
    (:3
      (LocalVariables|SetRoomRotation "0,270.000000, 0")))
  (bind _roomtype (CallFunction|PickRoomType))
  (Game|SpawnActorfromClass _roomtype (Math|Transform|MakeTransform _output_get (LocalVariables|GetRoomRotation) "1.000000,1.000000,1.000000") "Undefined" 0 0)
  (Variables|Default|SetLastRoomDirection "Right"))

(fn SpawnLeftRoom
  (bind _tilesize (Variables|Default|GetTileSize))
  (if (Variables|Default|GetIsFirstRoom)
    (LocalVariables|SetStartDoor 2)
    (Variables|Default|SetIsFirstRoom false)
    (else
      (LocalVariables|SetStartDoor (Math|Random|RandomIntegerinRange 1 3))))
  (LocalVariables|SetEndDoor (Math|Random|RandomIntegerinRange 1 3))
  (CallFunction|PickHallwayType (LocalVariables|GetStartDoor) (LocalVariables|GetEndDoor))
  (Variables|Default|SetHallwaySpawnPos (+ (Variables|Default|GetCurrentRoomPos) (Math|Vector|MakeVector (+ (* _tilesize -0.5) (* _tilesize (- (LocalVariables|GetStartDoor) 2))) (* (Variables|Default|GetTileSize) -1.5) 0.0)))
  (bind _output_get (Variables|Default|SetCurrentRoomPos (+ (Math|Vector|MakeVector (.x (Variables|Default|GetCurrentRoomPos)) (.y (Variables|Default|GetCurrentRoomPos)) 0.0) (Math|Vector|MakeVector 0.0 (* (* (Variables|Default|GetTileSize) (+ (Variables|Default|GetHallwaySize) 3.0)) -1.0) (/ (* (Variables|Grid|GetHeightOffset) (Math|Random|RandomIntegerinRange -1 1)) (Math|Random|RandomIntegerinRange 1 2))))))
  (switch int (Math|Random|RandomIntegerinRange 0 3)
    (:0
      (LocalVariables|SetRoomRotation "0, 0, 0"))
    (:1
      (LocalVariables|SetRoomRotation "0,90.000000, 0"))
    (:2
      (LocalVariables|SetRoomRotation "0,180.000000, 0"))
    (:3
      (LocalVariables|SetRoomRotation "0,270.000000, 0")))
  (bind _roomtype (CallFunction|PickRoomType))
  (Game|SpawnActorfromClass _roomtype (Math|Transform|MakeTransform _output_get (LocalVariables|GetRoomRotation) "1.000000,1.000000,1.000000") "Undefined" 0 0)
  (Variables|Default|SetLastRoomDirection "Left"))

(fn SpawnBackRoom
  (bind _tilesize (Variables|Default|GetTileSize))
  (if (Variables|Default|GetIsFirstRoom)
    (LocalVariables|SetStartDoor 2)
    (Variables|Default|SetIsFirstRoom false)
    (else
      (LocalVariables|SetStartDoor (Math|Random|RandomIntegerinRange 1 3))))
  (LocalVariables|SetEndDoor (Math|Random|RandomIntegerinRange 1 3))
  (CallFunction|PickHallwayType (LocalVariables|GetStartDoor) (LocalVariables|GetEndDoor))
  (Variables|Default|SetHallwaySpawnPos (+ (Variables|Default|GetCurrentRoomPos) (Math|Vector|MakeVector (* (Variables|Default|GetTileSize) -1.5) (+ (* _tilesize 0.5) (* _tilesize (* (- (LocalVariables|GetStartDoor) 2) -1.0))) 0.0)))
  (bind _output_get (Variables|Default|SetCurrentRoomPos (+ (Math|Vector|MakeVector (.x (Variables|Default|GetCurrentRoomPos)) (.y (Variables|Default|GetCurrentRoomPos)) 0.0) (Math|Vector|MakeVector (* (* (Variables|Default|GetTileSize) (+ (Variables|Default|GetHallwaySize) 3.0)) -1.0) 0.0 (/ (* (Variables|Grid|GetHeightOffset) (Math|Random|RandomIntegerinRange -1 1)) (Math|Random|RandomIntegerinRange 1 2))))))
  (switch int (Math|Random|RandomIntegerinRange 0 3)
    (:0
      (LocalVariables|SetRoomRotation "0, 0, 0"))
    (:1
      (LocalVariables|SetRoomRotation "0,90.000000, 0"))
    (:2
      (LocalVariables|SetRoomRotation "0,180.000000, 0"))
    (:3
      (LocalVariables|SetRoomRotation "0,270.000000, 0")))
  (bind _roomtype (CallFunction|PickRoomType))
  (Game|SpawnActorfromClass _roomtype (Math|Transform|MakeTransform _output_get (LocalVariables|GetRoomRotation) "1.000000,1.000000,1.000000") "Undefined" 0 0)
  (Variables|Default|SetLastRoomDirection "Back"))

(fn PickHallwayType
  (params (StartDoor :type Integer) (EndDoor :type Integer))
  (if (== StartDoor EndDoor)
    (Variables|Default|SetHallwayType "/Game/Blueprints/ProceduralGeneration_Levels/Hallways/BP_Hallway_V1.BP_Hallway_V1_C")
    (elif (or (and (== StartDoor 1) (== EndDoor 2)) (and (== StartDoor 2) (== EndDoor 3)))
      (Variables|Default|SetHallwayType "/Game/Blueprints/ProceduralGeneration_Levels/Hallways/BP_Hallway_V2.BP_Hallway_V2_C")
      (elif (and (== StartDoor 1) (== EndDoor 3))
        (Variables|Default|SetHallwayType "/Game/Blueprints/ProceduralGeneration_Levels/Hallways/BP_Hallway_V3.BP_Hallway_V3_C")
        (elif (or (and (== StartDoor 2) (== EndDoor 1)) (and (== StartDoor 3) (== EndDoor 2)))
          (Variables|Default|SetHallwayType "/Game/Blueprints/ProceduralGeneration_Levels/Hallways/BP_Hallway_V4.BP_Hallway_V4_C")
          (elif (and (== StartDoor 3) (== EndDoor 1))
            (Variables|Default|SetHallwayType "/Game/Blueprints/ProceduralGeneration_Levels/Hallways/BP_Hallway_V5.BP_Hallway_V5_C")
            (else
              (Development|PrintString "Appropriate Hallway Not Found!"))))))))

(fn PickRoomType
  (if (Math|Boolean|ORBoolean (!= (Variables|RoomTypes|GetNumOfRoom1) 0) (!= (Variables|RoomTypes|GetNumOfRoom2) 0) (!= (Variables|RoomTypes|GetNumOfRoom3) 0))
    _
    (else
      _))
  (return "/Game/Blueprints/ProceduralGeneration_Levels/BP_Room_Parent.BP_Room_Parent_C"))

(fn CreateLastHallway
  (bind _tilesize (Variables|Default|GetTileSize))
  (LocalVariables|SetStartDoor (Math|Random|RandomIntegerinRange 1 3))
  (LocalVariables|SetEndDoor (Math|Random|RandomIntegerinRange 1 3))
  (CallFunction|PickHallwayType (LocalVariables|GetStartDoor) (LocalVariables|GetEndDoor))
  (bind _output_get (Variables|Default|SetHallwaySpawnPos (+ (Variables|Default|GetCurrentRoomPos) (Math|Vector|MakeVector (+ (* _tilesize -0.5) (* _tilesize (- (LocalVariables|GetStartDoor) 2))) (* (Variables|Default|GetTileSize) -1.5) 0.0))))
  (Game|SpawnActorfromClass (Variables|Default|GetHallwayType) (Math|Transform|MakeTransform _output_get "0,-90.000000, 0" "1.000000,1.000000,1.000000") "Undefined" 0 0))

(fn ReplaceRooms
  (bind _outactors (Actor|GetAllActorsOfClass "/Game/Blueprints/ProceduralGeneration_Levels/BP_Room_Parent.BP_Room_Parent_C"))
  (LocalVariables|SetRoomArray _outactors)
  (if (< (Variables|RoomStats|GetTotalRooms) (Variables|RoomStats|GetExtraRooms))
    (Variables|RoomStats|SetExtraRooms (Variables|RoomStats|GetTotalRooms)))
  (Utilities|Array|Clear (LocalVariables|GetReplacedRoomArray))
  (Utilities|Array|Shuffle (LocalVariables|GetRoomArray))
  (for _index (range 1 (Variables|RoomStats|GetExtraRooms))
    (Utilities|Array|Add (LocalVariables|GetReplacedRoomArray) (Utilities|Array|Get(acopy) (LocalVariables|GetRoomArray) (- _index 1))))
  (for _array_element (LocalVariables|GetReplacedRoomArray)
    (bind _output_get (LocalVariables|SetReplacedRoomRef _array_element))
    (LocalVariables|SetReplacedRoomTransform (Transformation|GetActorTransform _output_get))
    (bind _output_get_2 (LocalVariables|SetRandomRoomType (Math|Random|RandomIntegerinRange 1 3) :!label _label))
    (if (and (== _output_get_2 1) (> (Variables|RoomTypes|GetNumOfRoom1) 0))
      (Game|SpawnActorfromClass "/Game/Blueprints/ProceduralGeneration_Levels/BP_Room_V1.BP_Room_V1_C" (LocalVariables|GetReplacedRoomTransform) "Undefined" 0 0)
      (Math|Integer|DecrementInt (Variables|RoomTypes|GetNumOfRoom1)
        (:%20%20
          _))
      (elif (and (== (LocalVariables|GetRandomRoomType) 2) (> (Variables|RoomTypes|GetNumOfRoom2) 0))
        (Game|SpawnActorfromClass "/Game/Blueprints/ProceduralGeneration_Levels/BP_Room_V2.BP_Room_V2_C" (LocalVariables|GetReplacedRoomTransform) "Undefined" 0 0)
        (Math|Integer|DecrementInt (Variables|RoomTypes|GetNumOfRoom2)
          (:%20%20
            _))
        (elif (and (== (LocalVariables|GetRandomRoomType) 3) (> (Variables|RoomTypes|GetNumOfRoom3) 0))
          (Game|SpawnActorfromClass "/Game/Blueprints/ProceduralGeneration_Levels/BP_Room_V3.BP_Room_V3_C" (LocalVariables|GetReplacedRoomTransform) "Undefined" 0 0)
          (Math|Integer|DecrementInt (Variables|RoomTypes|GetNumOfRoom3)
            (:%20%20
              _))
          (else
            (goto _label)))))
    (Actor|DestroyActor (LocalVariables|GetReplacedRoomRef))))

(fn DeleteRooms
  (bind _outactors (Actor|GetAllActorsOfClass "/Game/Blueprints/ProceduralGeneration_Levels/BP_Room_Parent.BP_Room_Parent_C"))
  (LocalVariables|SetRoomArray _outactors)
  (if (< (Variables|RoomStats|GetTotalRooms) (Variables|RoomStats|GetDeletedRooms))
    (Variables|RoomStats|SetDeletedRooms (Variables|RoomStats|GetTotalRooms)))
  (Utilities|Array|Clear (LocalVariables|GetDeletedRoomsArray))
  (Utilities|Array|Shuffle (LocalVariables|GetRoomArray))
  (for _index (range 1 (Variables|RoomStats|GetDeletedRooms))
    (Utilities|Array|Add (LocalVariables|GetDeletedRoomsArray) (Utilities|Array|Get(acopy) (LocalVariables|GetRoomArray) (- _index 1))))
  (for _array_element (LocalVariables|GetDeletedRoomsArray)
    (Actor|DestroyActor _array_element)))

(fn MoveSpawn
  (bind _outactors (Actor|GetAllActorsOfClass "/Game/Blueprints/ProceduralGeneration_Levels/BP_Room_Parent.BP_Room_Parent_C"))
  (LocalVariables|SetRoomArray _outactors)
  (Game|SpawnActorfromClass "/Game/Blueprints/ProceduralGeneration_Levels/BP_Room_Parent.BP_Room_Parent_C" (Transformation|GetActorTransform) "Undefined" 0 0)
  (Transformation|SetActorTransform (Math|Transform|MakeTransform (Math|Vector|MakeVector (.x (.location (Transformation|GetActorTransform (.OutItem (Utilities|Array|Random (LocalVariables|GetRoomArray)))))) (.y (.location (Transformation|GetActorTransform (.OutItem (Utilities|Array|Random (LocalVariables|GetRoomArray)))))) (+ (.z (.location (Transformation|GetActorTransform (.OutItem (Utilities|Array|Random (LocalVariables|GetRoomArray)))))) (Variables|Default|GetSpawnHeightOffset))) "0, 0, 0" "1.000000,1.000000,1.000000")))