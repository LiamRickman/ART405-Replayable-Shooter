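; Procedural level generator that spawns a chain of rooms joined by hallways on BeginPlay.
; Each step picks a direction that avoids reversing the last, then advances a tile-based position cursor without checking for overlaps.
; Random start and end door slots select one of five hallway variants to bridge the offset.
; Rooms get random quarter-turn rotations, with types drawn by rerolling against remaining per-type quotas.
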(event EventBeginPlay
  (bind _output_get (Variables|Default|SetTotalRooms (+ (Variables|RoomTypes|GetNumOfFillerRooms) (Variables|RoomTypes|GetNumOfRoom1) (Variables|RoomTypes|GetNumOfRoom2) (Variables|RoomTypes|GetNumOfRoom3))))
  (for _index (range 1 _output_get)
    (if (Variables|Default|GetIsFirstRoom)
      (switch int (Math|Random|RandomIntegerinRange 0 1)
        (:0
          (CallFunction|SpawnFrontRoom))
        (:1
          (CallFunction|SpawnBackRoom)))
      (else
        (switch string (Variables|Default|GetLastRoomDirection)
          (:Front
            (switch int (Math|Random|RandomInteger 2)
              (:0
                (CallFunction|SpawnFrontRoom))
              (:1
                (CallFunction|SpawnLeftRoom))
              (:2
                (CallFunction|SpawnRightRoom))))
          (:Back
            (switch int (Math|Random|RandomInteger 2)
              (:0
                (CallFunction|SpawnBackRoom))
              (:1
                (CallFunction|SpawnLeftRoom))
              (:2
                (CallFunction|SpawnRightRoom))))
          (:Left
            (switch int (Math|Random|RandomInteger 2)
              (:0
                (CallFunction|SpawnFrontRoom))
              (:1
                (CallFunction|SpawnBackRoom))
              (:2
                (CallFunction|SpawnRightRoom))))
          (:Right
            (switch int (Math|Random|RandomInteger 2)
              (:0
                (CallFunction|SpawnFrontRoom))
              (:1
                (CallFunction|SpawnLeftRoom))
              (:2
                (CallFunction|SpawnBackRoom)))))))))

(fn ConstructionScript)

(fn SpawnFrontRoom
  (bind _tilesize (Variables|Default|GetTileSize))
  (if (Variables|Default|GetIsFirstRoom)
    (LocalVariables|SetStartDoor 2)
    (Variables|Default|SetIsFirstRoom false)
    (else
      (LocalVariables|SetStartDoor (Math|Random|RandomIntegerinRange 1 3))))
  (LocalVariables|SetEndDoor (Math|Random|RandomIntegerinRange 1 3))
  (CallFunction|PickHallwayType (LocalVariables|GetStartDoor) (LocalVariables|GetEndDoor))
  (bind _roomtype (CallFunction|PickRoomType))
  (Variables|Default|SetRoomType _roomtype)
  (Variables|Default|SetHallwaySpawnPos (+ (Variables|Default|GetCurrentRoomPos) (Math|Vector|MakeVector (* (Variables|Default|GetTileSize) 1.5) (+ (* _tilesize -1.0) (* _tilesize (- (LocalVariables|GetStartDoor) 1))) 0.0)))
  (bind _output_get (Variables|Default|SetCurrentRoomPos (+ (Variables|Default|GetCurrentRoomPos) (Math|Vector|MakeVector (* (Variables|Default|GetTileSize) (+ (Variables|Default|GetHallwaySize) 3.0)) 0.0 0.0))))
  (switch int (Math|Random|RandomIntegerinRange 0 3)
    (:0
      (LocalVariables|SetRoomRotation "0, 0, 0"))
    (:1
      (LocalVariables|SetRoomRotation "0,90.000000, 0"))
    (:2
      (LocalVariables|SetRoomRotation "0,180.000000, 0"))
    (:3
      (LocalVariables|SetRoomRotation "0,270.000000, 0")))
  (Game|SpawnActorfromClass (Variables|Default|GetRoomType) (Math|Transform|MakeTransform _output_get (LocalVariables|GetRoomRotation) "1.000000,1.000000,1.000000") "Undefined" 0 0)
  (Game|SpawnActorfromClass (Variables|Default|GetHallwayType) (Math|Transform|MakeTransform (Variables|Default|GetHallwaySpawnPos) "0, 0, 0" "1.000000,1.000000,1.000000") "Undefined" 0 0)
  (Variables|Default|SetLastRoomDirection "Front"))

(fn SpawnRightRoom
  (bind _tilesize (Variables|Default|GetTileSize))
  (if (Variables|Default|GetIsFirstRoom)
    (LocalVariables|SetStartDoor 2)
    (Variables|Default|SetIsFirstRoom false)
    (else
      (LocalVariables|SetStartDoor (Math|Random|RandomIntegerinRange 1 3))))
  (LocalVariables|SetEndDoor (Math|Random|RandomIntegerinRange 1 3))
  (CallFunction|PickHallwayType (LocalVariables|GetStartDoor) (LocalVariables|GetEndDoor))
  (Variables|Default|SetHallwaySpawnPos (+ (Variables|Default|GetCurrentRoomPos) (Math|Vector|MakeVector (+ (* _tilesize 1.0) (* _tilesize (* (- (LocalVariables|GetStartDoor) 1) -1))) (* (Variables|Default|GetTileSize) 1.5) 0.0)))
  (bind _output_get (Variables|Default|SetCurrentRoomPos (+ (Variables|Default|GetCurrentRoomPos) (Math|Vector|MakeVector 0.0 (* (Variables|Default|GetTileSize) (+ (Variables|Default|GetHallwaySize) 3.0)) 0.0))))
  (switch int (Math|Random|RandomIntegerinRange 0 3)
    (:0
      (LocalVariables|SetRoomRotation "0, 0, 0"))
    (:1
      (LocalVariables|SetRoomRotation "0,90.000000, 0"))
    (:2
      (LocalVariables|SetRoomRotation "0,180.000000, 0"))
    (:3
      (LocalVariables|SetRoomRotation "0,270.000000, 0")))
  (bind _roomtype (CallFunction|PickRoomType))
  (Game|SpawnActorfromClass _roomtype (Math|Transform|MakeTransform _output_get (LocalVariables|GetRoomRotation) "1.000000,1.000000,1.000000") "Undefined" 0 0)
  (Game|SpawnActorfromClass (Variables|Default|GetHallwayType) (Math|Transform|MakeTransform (Variables|Default|GetHallwaySpawnPos) "0,90.000000, 0" "1.000000,1.000000,1.000000") "Undefined" 0 0)
  (Variables|Default|SetLastRoomDirection "Right"))

(fn SpawnLeftRoom
  (bind _tilesize (Variables|Default|GetTileSize))
  (if (Variables|Default|GetIsFirstRoom)
    (LocalVariables|SetStartDoor 2)
    (Variables|Default|SetIsFirstRoom false)
    (else
      (LocalVariables|SetStartDoor (Math|Random|RandomIntegerinRange 1 3))))
  (LocalVariables|SetEndDoor (Math|Random|RandomIntegerinRange 1 3))
  (CallFunction|PickHallwayType (LocalVariables|GetStartDoor) (LocalVariables|GetEndDoor))
  (Variables|Default|SetHallwaySpawnPos (+ (Variables|Default|GetCurrentRoomPos) (Math|Vector|MakeVector (+ (* _tilesize -1.0) (* _tilesize (- (LocalVariables|GetStartDoor) 1))) (* (Variables|Default|GetTileSize) -1.5) 0.0)))
  (bind _output_get (Variables|Default|SetCurrentRoomPos (+ (Variables|Default|GetCurrentRoomPos) (Math|Vector|MakeVector 0.0 (* (* (Variables|Default|GetTileSize) (+ (Variables|Default|GetHallwaySize) 3.0)) -1.0) 0.0))))
  (switch int (Math|Random|RandomIntegerinRange 0 3)
    (:0
      (LocalVariables|SetRoomRotation "0, 0, 0"))
    (:1
      (LocalVariables|SetRoomRotation "0,90.000000, 0"))
    (:2
      (LocalVariables|SetRoomRotation "0,180.000000, 0"))
    (:3
      (LocalVariables|SetRoomRotation "0,270.000000, 0")))
  (bind _roomtype (CallFunction|PickRoomType))
  (Game|SpawnActorfromClass _roomtype (Math|Transform|MakeTransform _output_get (LocalVariables|GetRoomRotation) "1.000000,1.000000,1.000000") "Undefined" 0 0)
  (Game|SpawnActorfromClass (Variables|Default|GetHallwayType) (Math|Transform|MakeTransform (Variables|Default|GetHallwaySpawnPos) "0,-90.000000, 0" "1.000000,1.000000,1.000000") "Undefined" 0 0)
  (Variables|Default|SetLastRoomDirection "Left"))

(fn SpawnBackRoom
  (bind _tilesize (Variables|Default|GetTileSize))
  (if (Variables|Default|GetIsFirstRoom)
    (LocalVariables|SetStartDoor 2)
    (Variables|Default|SetIsFirstRoom false)
    (else
      (LocalVariables|SetStartDoor (Math|Random|RandomIntegerinRange 1 3))))
  (LocalVariables|SetEndDoor (Math|Random|RandomIntegerinRange 1 3))
  (CallFunction|PickHallwayType (LocalVariables|GetStartDoor) (LocalVariables|GetEndDoor))
  (Variables|Default|SetHallwaySpawnPos (+ (Variables|Default|GetCurrentRoomPos) (Math|Vector|MakeVector (* (Variables|Default|GetTileSize) -1.5) (+ (* _tilesize 1.0) (* _tilesize (* (- (LocalVariables|GetStartDoor) 1) -1.0))) 0.0)))
  (bind _output_get (Variables|Default|SetCurrentRoomPos (+ (Variables|Default|GetCurrentRoomPos) (Math|Vector|MakeVector (* (* (Variables|Default|GetTileSize) (+ (Variables|Default|GetHallwaySize) 3.0)) -1.0) 0.0 0.0))))
  (switch int (Math|Random|RandomIntegerinRange 0 3)
    (:0
      (LocalVariables|SetRoomRotation "0, 0, 0"))
    (:1
      (LocalVariables|SetRoomRotation "0,90.000000, 0"))
    (:2
      (LocalVariables|SetRoomRotation "0,180.000000, 0"))
    (:3
      (LocalVariables|SetRoomRotation "0,270.000000, 0")))
  (bind _roomtype (CallFunction|PickRoomType))
  (Game|SpawnActorfromClass _roomtype (Math|Transform|MakeTransform _output_get (LocalVariables|GetRoomRotation) "1.000000,1.000000,1.000000") "Undefined" 0 0)
  (Game|SpawnActorfromClass (Variables|Default|GetHallwayType) (Math|Transform|MakeTransform (Variables|Default|GetHallwaySpawnPos) "0,180.000000, 0" "1.000000,1.000000,1.000000") "Undefined" 0 0)
  (Variables|Default|SetLastRoomDirection "Back"))

(fn PickHallwayType
  (params (StartDoor :type Integer) (EndDoor :type Integer))
  (if (== StartDoor EndDoor)
    (Variables|Default|SetHallwayType "/Game/Blueprints/ProceduralGeneration_Levels/Hallways/BP_Hallway_V1.BP_Hallway_V1_C")
    (elif (or (and (== StartDoor 1) (== EndDoor 2)) (and (== StartDoor 2) (== EndDoor 3)))
      (Variables|Default|SetHallwayType "/Game/Blueprints/ProceduralGeneration_Levels/Hallways/BP_Hallway_V2.BP_Hallway_V2_C")
      (elif (and (== StartDoor 1) (== EndDoor 3))
        (Variables|Default|SetHallwayType "/Game/Blueprints/ProceduralGeneration_Levels/Hallways/BP_Hallway_V3.BP_Hallway_V3_C")
        (elif (or (and (== StartDoor 2) (== EndDoor 1)) (and (== StartDoor 3) (== EndDoor 2)))
          (Variables|Default|SetHallwayType "/Game/Blueprints/ProceduralGeneration_Levels/Hallways/BP_Hallway_V4.BP_Hallway_V4_C")
          (elif (and (== StartDoor 3) (== EndDoor 1))
            (Variables|Default|SetHallwayType "/Game/Blueprints/ProceduralGeneration_Levels/Hallways/BP_Hallway_V5.BP_Hallway_V5_C")
            (else
              (Development|PrintString "Appropriate Hallway Not Found!"))))))))

(fn PickRoomType
  (if (Math|Boolean|ORBoolean (!= (Variables|RoomTypes|GetNumOfRoom1) 0) (!= (Variables|RoomTypes|GetNumOfRoom2) 0) (!= (Variables|RoomTypes|GetNumOfRoom3) 0))
    (switch int (Math|Random|RandomIntegerinRange 0 3) :!label _label
      (:0
        (if (> (Variables|RoomTypes|GetNumOfFillerRooms) 0)
          (Math|Integer|DecrementInt (Variables|RoomTypes|GetNumOfFillerRooms)
            (:%20%20
              (return "/Game/Blueprints/ProceduralGeneration_Levels/BP_Room_Parent.BP_Room_Parent_C")))
          (else
            (goto _label))))
      (:1
        (if (> (Variables|RoomTypes|GetNumOfRoom1) 0)
          (Math|Integer|DecrementInt (Variables|RoomTypes|GetNumOfRoom1)
            (:%20%20
              (return "/Game/Blueprints/ProceduralGeneration_Levels/BP_Room_V1.BP_Room_V1_C")))
          (else
            (goto _label))))
      (:2
        (if (> (Variables|RoomTypes|GetNumOfRoom2) 0)
          (Math|Integer|DecrementInt (Variables|RoomTypes|GetNumOfRoom2)
            (:%20%20
              (return "/Game/Blueprints/ProceduralGeneration_Levels/BP_Room_V2.BP_Room_V2_C")))
          (else
            (goto _label))))
      (:3
        (if (> (Variables|RoomTypes|GetNumOfRoom3) 0)
          (Math|Integer|DecrementInt (Variables|RoomTypes|GetNumOfRoom3)
            (:%20%20
              (return "/Game/Blueprints/ProceduralGeneration_Levels/BP_Room_V3.BP_Room_V3_C")))
          (else
            (goto _label)))))
    (else
      (return "/Game/Blueprints/ProceduralGeneration_Levels/BP_Room_Parent.BP_Room_Parent_C"))))